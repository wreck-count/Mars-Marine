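; Alien enemy pawn that chases the player character and attacks within range.
; An AI MoveTo loop re-issues while alive; Tick halts movement and plays the attack montage in range, restoring movement on completion.
; DamagePlayer applies hit damage but is not called within this Blueprint.
; Damage lowers clamped HP; at zero it disables collision and movement, credits the marine's kill, notifies the game mode, then destroys itself after a delay.
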(event `self.ReceiveBeginPlay`
  (`|AIMoveTo` self (0.0 0.0 0.0) (`GameplayStatics.GetPlayerCharacter` 0) :!label _label
    (:`OnSuccess`
      _)
    (:`OnFail`
      _))
  (`KismetSystemLibrary.Delay` 0.2)
  (if (`self.Alive`)
    (goto _label)))

(event `self.ReceiveTick`
  (params (DeltaSeconds :type "Float (single-precision)"))
  (if (and (`self.IsWithinPlayerRange`) (not (`self.IsAttacking`)) (`self.Alive`))
    (`self.Deactivate AIMovement`)
    (`|PlayMontage` (`self.Mesh`) "/Game/Characters/Enemy_Great_Spider/Animations/AlienAttackMontage.AlienAttackMontage"
      (:`OnCompleted`
        (`self.ActivateAIMovement`)))))

(event `self.ReceiveAnyDamage`
  (params (Damage :type "Float (single-precision)") (DamageType :type "DamageType Object Reference") (InstigatedBy :type "Controller Object Reference") (DamageCauser :type "Actor Object Reference"))
  (if (`self.Alive`)
    (`self.DecreaseHP` Damage)
    (if (== (`self.AlienHP`) 0.0)
      (`self.KillAI`)
      (`KismetSystemLibrary.Delay` 3.0)
      (`self.K2_DestroyActor`))))

(fn `ActivateAIMovement`
  (`ActorComponent.Activate` (`self.CharacterMovement`) false))

(fn `DamagePlayer`
  (`GameplayStatics.ApplyDamage` (`GameplayStatics.GetPlayerCharacter` 0) (`self.DamagePerHit`)))

(fn `Deactivate AIMovement`
  (bind _charactermovement (`self.CharacterMovement`))
  (`MovementComponent.StopMovementImmediately` _charactermovement)
  (`ActorComponent.Deactivate` _charactermovement))

(fn `DecreaseHP`
  (params (DamageReceived :type "Float (double-precision)"))
  (set `self.AlienHP` (`KismetMathLibrary.FClamp` (- (`self.AlienHP`) DamageReceived) 0.0 200.0)))

(fn `IsAlive`
  (returns (Alive :type Boolean))
  (return (`self.Alive`)))

(fn `IsAttacking`
  (returns (ReturnValue :type Boolean))
  (return (`AnimInstance.Montage_IsPlaying` (`SkeletalMeshComponent.GetAnimInstance` (`self.Mesh`)) "/Game/Characters/Enemy_Great_Spider/Animations/AlienAttackMontage.AlienAttackMontage")))

(fn `IsWithinPlayerRange`
  (returns (ReturnValue :type Boolean))
  (return (<= (`self.GetDistanceTo` (`GameplayStatics.GetPlayerCharacter` 0)) (`self.AttackRange`))))

(fn `KillAI`
  (set `self.Alive` false)
  (`self.Deactivate AIMovement`)
  (`self.SetActorEnableCollision` false)
  (bind _asbp_mars_marine (cast `/Game/Blueprints/Pawns/BP_MarsMarine` (`GameplayStatics.GetPlayerCharacter` 0)))
  (`/Game/Blueprints/Pawns/BP_MarsMarine.IncreaseKills` _asbp_mars_marine)
  (bind _asbp_game_mode (cast `/Game/Blueprints/GameMode/BP_GameMode` (`GameplayStatics.GetGameMode`)))
  (`/Game/Blueprints/GameMode/BP_GameMode.RegisterAlienDeath` _asbp_game_mode self))

(fn `UserConstructionScript`)