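; Game mode that runs escalating waves of alien enemies.
; Each wave scales the previous spawn count by a difficulty multiplier, then a looping timer spawns BP_Alien actors at random TargetPoints until the count runs out.
; Living aliens are tracked in an array, and RegisterAlienDeath removes them.
; When none remain alive or waiting to spawn, the next wave starts after a short delay.
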(event `self.ReceiveBeginPlay`
  (`KismetSystemLibrary.Delay` 2.0)
  (`self.SetupNextWave`))

(event `Spawn Wave`
  (`self.SpawnAlien`))

(event `EndWave`
  (`KismetSystemLibrary.Delay` 2.0)
  (`self.SetupNextWave`))

(fn `GetRandomSpawnPoint`
  (returns (ReturnValue :type "TargetPoint Object Reference"))
  (bind _outactors (`GameplayStatics.GetAllActorsOfClass` "/Script/Engine.TargetPoint"))
  (return (`|GetArrayItem` _outactors (`KismetMathLibrary.RandomIntegerInRange` 0 (`KismetArrayLibrary.Array_LastIndex` _outactors)))))

(fn `IsWaveOver`
  (returns (ReturnValue :type Boolean))
  (return (and (== (`KismetArrayLibrary.Array_Length` (`self.Aliens`)) 0) (== (`self.CurAliensToSpawn`) 0))))

(fn `RegisterAlienDeath`
  (params (Item :type "/Game/Blueprints/Pawns/BP_Alien Object Reference (by ref)"))
  (`KismetArrayLibrary.Array_RemoveItem` (`self.Aliens`) Item)
  (if (`self.IsWaveOver`)
    (`self.EndWave`)))

(fn `SetDifficultyWithWave`
  (bind _output_get (set `self.CurAliensToSpawn` (`KismetMathLibrary.Round` (* (`self.PrevAlienToSpawn`) (`self.DifficultyMultiplier`)))))
  (set `self.PrevAlienToSpawn` _output_get))

(fn `SetupNextWave`
  (`/Engine/EditorBlueprintResources/StandardMacros.IncrementInt` (`self.CurrentWave`)
    (:`  `
      (`self.SetDifficultyWithWave`)
      (`KismetSystemLibrary.K2_SetTimer` null "Spawn Wave" 1.0 true))))

(fn `SpawnAlien`
  (bind _returnvalue (`self.GetRandomSpawnPoint`))
  (`/Engine/EditorBlueprintResources/StandardMacros.IsValid` _returnvalue
    (:`Is Valid`
      (bind _returnvalue_2 (`|SpawnActorFromClass` "/Game/Blueprints/Pawns/BP_Alien.BP_Alien_C" (`self.GetTransform` _returnvalue) "Undefined" "OverrideRootScale" null null))
      (`/Engine/EditorBlueprintResources/StandardMacros.IsValid` _returnvalue_2
        (:`Is Valid`
          (`KismetArrayLibrary.Array_Add` (`self.Aliens`) _returnvalue_2)
          (bind _result (`/Engine/EditorBlueprintResources/StandardMacros.DecrementInt` (`self.CurAliensToSpawn`))
            (:`  `
              (if (== _result 0)
                (`KismetSystemLibrary.K2_ClearTimer` null "Spawn Wave")))))))))

(fn `UserConstructionScript`)